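; BP_Chaser is an AI character that can attack and choose patrol points.
; Its Attack event forwards an AttackMessage to the mesh's anim instance when that instance is valid.
; GetRandomPatrolLocation lives on the character so patrol locations can be saved per placed instance.
; It draws random entries separately for comparison and assignment, so CurrentPoint can repeat, and it assigns and returns only when the compared draw differs.
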(event `/Game/Custom/AI/BPI_Attack.Attack`
  (bind _returnvalue (`SkeletalMeshComponent.GetAnimInstance` (`self.Mesh`)))
  (`/Engine/EditorBlueprintResources/StandardMacros.IsValid` _returnvalue
    (:`Is Valid`
      (message `/Game/Custom/AI/BPI_Attack.Attack` _returnvalue))))

(fn `GetRandomPatrolLocation`
  (returns (TargetPoint :type "TargetPoint Object Reference"))
  (bind _outitem (`KismetArrayLibrary.Array_Random` (`self.PatrolLocations`)))
  ;[1 1 1] This needs to stay in character as controller cannot be placed and save predetermined variable in the world.
  (if (!= _outitem (`self.CurrentPoint`))
    (bind _output_get (set `self.CurrentPoint` _outitem))
    (return _output_get)))

(fn `UserConstructionScript`)