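; AI controller for a chaser enemy that runs the BT_Chaser behavior tree on BeginPlay.
; AI perception updates feed HandleSightSense, which filters for sight stimuli on the player character.
; A match writes the actor to the Player blackboard key and sets LastKnownLocation to a zero vector, using literal key names.
; It does not check whether sight was gained or lost.
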(event `self.ReceiveBeginPlay`
  (`self.RunBehaviorTree` "/Game/Custom/AI/BT_Chaser.BT_Chaser"))

(event `self.AIPerception.OnTargetPerceptionUpdated`
  (params (Actor :type "Actor Object Reference") (Stimulus :type "AIStimulus Structure"))
  ;[1 1 1] This event is called whenever the perception is updated
  (`self.HandleSightSense` Actor Stimulus))

(fn `HandleSightSense`
  (params (SightedActor :type "Actor Object Reference") (Stimulus :type "AIStimulus Structure"))
  ;[1 1 1] As stimulus comes in many form such as sight, hearing and more. We need t filter those first before handling
  (bind _returnvalue (`AIPerceptionSystem.GetSenseClassForStimulus` Stimulus))
  (if (== _returnvalue "/Script/AIModule.AISense_Sight")
    (if (== (`local.SightedActor`) (`GameplayStatics.GetPlayerCharacter` 0))
      ;[1 1 1] Criticism: By referencing to blackboard directly and using literal name of magic variable, it can lead to unexpected behavior.
      (`BlackboardComponent.SetValueAsObject` (`self.Blackboard`) "Player" (`local.SightedActor`))
      (`BlackboardComponent.SetValueAsVector` (`self.Blackboard`) "LastKnownLocation" (0.0 0.0 0.0))
      (else
        (return)))
    (else
      (return))))

(fn `UserConstructionScript`)