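; BP_InteractableBox is a base interactable actor that shows a text prompt while the player's interaction line-of-sight actor overlaps its box.
; The prompt stays visible in the editor for labeling and hides at BeginPlay.
; The Interact event calls an overridable Interacts function, which child classes replace to avoid duplicated interface code.
; One-time interactables then hide themselves and disable box collision.
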(event `/Game/Custom/Interactable/BPI_Interactable.Interact`
  (`self.Interacts`)
  (if (`self.IsOneTimeInteractable`)
    (`SceneComponent.SetVisibility` (`self.DefaultSceneRoot`) false true)
    (`PrimitiveComponent.SetCollisionEnabled` (`self.Box`) "NoCollision")))

(event `self.Box.OnComponentBeginOverlap`
  (params (OverlappedComponent :type "PrimitiveComponent Object Reference") (OtherActor :type "Actor Object Reference") (OtherComp :type "PrimitiveComponent Object Reference") (OtherBodyIndex :type Integer) (bFromSweep :type Boolean) (SweepResult :type "HitResult Structure (by ref)"))
  (if (== (`GameplayStatics.GetObjectClass` OtherActor) "/Game/Custom/Player/BP_InteractionLineOfSight.BP_InteractionLineOfSight_C")
    (`SceneComponent.SetVisibility` (`self.InteractText`) true false)))

(event `self.ReceiveBeginPlay`
  ;[1 1 1] Reason: As we have difference type of interaction point, we need to see their label in editing mode for ease of delvelopment
  (`SceneComponent.SetVisibility` (`self.InteractText`) false false))

(event `self.Box.OnComponentEndOverlap`
  (params (OverlappedComponent :type "PrimitiveComponent Object Reference") (OtherActor :type "Actor Object Reference") (OtherComp :type "PrimitiveComponent Object Reference") (OtherBodyIndex :type Integer))
  (if (== (`GameplayStatics.GetObjectClass` OtherActor) "/Game/Custom/Player/BP_InteractionLineOfSight.BP_InteractionLineOfSight_C")
    (`SceneComponent.SetVisibility` (`self.InteractText`) false false)))

(fn `Interacts`
  ;[1 1 1] This is just a empty function for its child to override. Trying to implement interface on children but it can result in duplicated codes.
  (`KismetSystemLibrary.PrintString` "This box is interacted"))

(fn `UserConstructionScript`)