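; BPC_Health is a player health component that tracks current and maximum health points.
; AddHealth and DecreaseHealth clamp the value between zero and the maximum, then fire increased or decreased dispatchers.
; DecreaseHealth also fires a zero-health dispatcher when health is empty.
; Debug Z and X key handlers and a health print event remain, but their input-enabling and dispatcher bindings are disconnected.
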(event Custom|OnHealtUpdate
  ;[1 0.8694 0.4268] For debugging only
  (Development|PrintString (Utilities|String|ToString(Text) (Utilities|Text|FormatText "Health is {Current}/{Max}" (Variables|Default|GetHealthPoint) (Variables|Default|GetMaxHealthPoint)))))

(event EventBeginPlay
  ;[1 0.8694 0.4268] For debugging only
)

(event Input|KeyboardEvents|DebugKeyX
  (params (Key :type Key%20Structure :default "None") (ActionValue :type Input%20Action%20Value%20Structure))
  ;[1 0.6664 0.4684] For debugging only
  (:Pressed
    (CallFunction|DecreaseHealth 1)))

(event Input|KeyboardEvents|DebugKeyZ
  (params (Key :type Key%20Structure :default "None") (ActionValue :type Input%20Action%20Value%20Structure))
  ;[1 0.6664 0.4684] For debugging only
  (:Pressed
    (CallFunction|AddHealth 1)))

(fn DecreaseHealth
  (params (AmountDecreased :type Integer))
  (bind _output_get (Variables|Default|SetHealthPoint (Math|Integer|Clamp(Integer) (- (Variables|Default|GetHealthPoint) AmountDecreased) 0 (Variables|Default|GetMaxHealthPoint))))
  (Default|CallOnHealthDecreased)
  (if (== _output_get 0)
    (Default|CallOnHealthIsZero)))

(fn AddHealth
  (params (AmountAdded :type Integer))
  (Variables|Default|SetHealthPoint (Math|Integer|Clamp(Integer) (+ AmountAdded (Variables|Default|GetHealthPoint)) 0 (Variables|Default|GetMaxHealthPoint)))
  (Default|CallOnHealthIncreased))