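; Player interaction actor that uses a collider to detect interactable actors and sends them an interact message on input.
; It enables input on BeginPlay and filters overlaps by the BPI_Interactable interface.
; Begin overlap adds a higher-priority Enhanced Input mapping context so interact overrides the flashlight toggle, and end overlap removes it to restore the flashlight.
; IA_Interact calls InteractMessage on the overlapped actor.
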(event `self.ReceiveBeginPlay`
  ;[1 1 1] Getting palyer controller for input action mapping contrext
  (`self.EnableInput` (`GameplayStatics.GetPlayerController` 0)))

(event `EnhancedInput|/Game/Custom/Inputs/IA_Interact`
  (params (ActionValue :type Boolean) (ElapsedSeconds :type "Float (double-precision)") (TriggeredSeconds :type "Float (double-precision)") (InputAction :type "InputAction Object Reference" :default "/Game/Custom/Inputs/IA_Interact.IA_Interact"))
  (:`Triggered`
    (message `/Game/Custom/Player/BPI_Interactable.Interact` (stale `self.Collider.OnComponentBeginOverlap` OtherActor))))

(event `self.Collider.OnComponentBeginOverlap`
  (params (OverlappedComponent :type "PrimitiveComponent Object Reference") (OtherActor :type "Actor Object Reference") (OtherComp :type "PrimitiveComponent Object Reference") (OtherBodyIndex :type Integer) (bFromSweep :type Boolean) (SweepResult :type "HitResult Structure (by ref)"))
  ;[1 1 1] Adding mapping context for interaction so that it will override flashlight toggling due to higher priority
  (if (`KismetSystemLibrary.DoesImplementInterface` OtherActor "/Game/Custom/Player/BPI_Interactable.BPI_Interactable_C")
    (`KismetSystemLibrary.PrintString` "This begin overlapped actor is interactable")
    (`EnhancedInputSubsystemInterface.AddMappingContext` (pcsubsystem `EnhancedInputLocalPlayerSubsystem` (`GameplayStatics.GetPlayerController` 0)) "/Game/Custom/Inputs/IMC_InteractableContext.IMC_InteractableContext" 1 (struct))))

(event `self.Collider.OnComponentEndOverlap`
  (params (OverlappedComponent :type "PrimitiveComponent Object Reference") (OtherActor :type "Actor Object Reference") (OtherComp :type "PrimitiveComponent Object Reference") (OtherBodyIndex :type Integer))
  (bind _returnvalue (pcsubsystem `EnhancedInputLocalPlayerSubsystem` (`GameplayStatics.GetPlayerController` 0)))
  (if (`KismetSystemLibrary.DoesImplementInterface` OtherActor "/Game/Custom/Player/BPI_Interactable.BPI_Interactable_C")
    (`KismetSystemLibrary.PrintString` "This end overlapped actor is interactable")
    ;[1 1 1] Removing context mapping when not in used. Else flashlight won't be usable after interactable for once.
    (`/Engine/EditorBlueprintResources/StandardMacros.IsValid` _returnvalue
      (:`Is Valid`
        (`EnhancedInputSubsystemInterface.RemoveMappingContext` _returnvalue "/Game/Custom/Inputs/IMC_InteractableContext.IMC_InteractableContext" (struct))))))

(fn `UserConstructionScript`)