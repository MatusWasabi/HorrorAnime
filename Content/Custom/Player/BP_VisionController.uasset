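; Player vision controller that acts as a battery-powered flashlight by switching the Fog blend weight between normal and maximum vision.
; BeginPlay takes maximum vision from the Fog's scene value and starts switched off; IA_ToggleFlashlight toggles it.
; Looping one-second timers, used instead of Tick, drain or recharge the battery and fire change callbacks.
; An empty battery forces the light off and blocks reopening until recharge reaches a fixed threshold.
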(event `self.ReceiveBeginPlay`
  ;[1 1 1] Setting base attenuation radius based on scene not blueprint class setting as it will be easier to test in scene for suitable brightness
  (set `self.MaximumVisionWeight` (`PostProcessComponent.BlendWeight` (`self.Fog`)))
  ;[1 1 1] Binding input for testing out its function without having to control it.
  (`self.EnableInput` (`GameplayStatics.GetPlayerController` 0))
  (`self.Close Light`))

(event `EnhancedInput|/Game/Custom/Inputs/IA_ToggleFlashlight`
  (params (ActionValue :type Boolean) (ElapsedSeconds :type "Float (double-precision)") (TriggeredSeconds :type "Float (double-precision)") (InputAction :type "InputAction Object Reference" :default "/Game/Custom/Inputs/IA_ToggleFlashlight.IA_ToggleFlashlight"))
  (:`Triggered`
    ;[1 1 1] Was a flip flop logic but failed to do as there are event when light is closed by other place outside player control.
    (if (`self.IsFlashlightOn`)
      (`self.Close Light`)
      (else
        (`self.Open Light`)))))

(event `DecreaseBattery`
  (bind _result (`/Engine/EditorBlueprintResources/StandardMacros.DecrementFloat` (`self.BatteryLevel`))
    (:`  `
      (`self.OnBatteryDecreased`)
      (if (== (`KismetMathLibrary.FClamp` _result 0.0 (`self.MaximumLevel`)) 0.0)
        (`self.Close Light`)
        (set `self.IsRecentlyDriedOut` true)))))

(event `IncreaseBattery`
  (bind _result (`/Engine/EditorBlueprintResources/StandardMacros.IncrementFloat` (`self.BatteryLevel`))
    (:`  `
      (`self.OnBatteryIncreased`)
      (if (>= (`KismetMathLibrary.FClamp` _result 0.0 (`self.MaximumLevel`)) 3.0)
        (`KismetSystemLibrary.K2_ClearAndInvalidateTimerHandle` (`self.Battery Increasing Timer`))
        (set `self.IsRecentlyDriedOut` false)))))

(fn `Close Light`
  (set `PostProcessComponent.BlendWeight` (`self.NormalVisionWeight`) (`self.Fog`))
  ;[1 1 1] Using timer instead of tick because tick is performance-heavied and many time messed up programming logic.
  (bind _returnvalue (`KismetSystemLibrary.K2_SetTimerDelegate` (`|CreateDelegate` :!event `IncreaseBattery`) 1.0 true))
  (set `self.Battery Increasing Timer` _returnvalue)
  ;[1 1 1] Clear timer here because both event called by timer should not be ran as same time as this function timer.
  (set `self.IsFlashlightOn` false)
  (`KismetSystemLibrary.K2_ClearAndInvalidateTimerHandle` (`self.Battery Decreasing Timer`)))

(fn `Open Light`
  ;[1 1 1] Clear timer due to this function timer and another must not happened at the same time.
  (if (not (`self.IsRecentlyDriedOut`))
    (`KismetSystemLibrary.K2_ClearAndInvalidateTimerHandle` (`self.Battery Increasing Timer`))
    (set `PostProcessComponent.BlendWeight` (`self.MaximumVisionWeight`) (`self.Fog`))
    (bind _returnvalue (`KismetSystemLibrary.K2_SetTimerDelegate` (`|CreateDelegate` :!event `DecreaseBattery`) 1.0 true))
    (set `self.Battery Decreasing Timer` _returnvalue)
    (set `self.IsFlashlightOn` true)))

(fn `UserConstructionScript`)